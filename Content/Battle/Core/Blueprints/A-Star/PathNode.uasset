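; PathNode is a node Blueprint for A-Star pathfinding in battle, holding its own grid coordinates and those of its parent.
; TraceToParent scales both coordinates to 100-unit cells and offsets them to cell centers at a height of 64.
; It runs a Visibility line trace between the two points, using only the timed debug draw to show the link, as the hit result is unused.
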(event `TraceToParent`
  (`KismetSystemLibrary.LineTraceSingle` :`Start` (+ (* (`KismetMathLibrary.MakeVector` (`KismetMathLibrary.Conv_IntToDouble` (`self.X`)) (`KismetMathLibrary.Conv_IntToDouble` (`self.Y`))) 100.0) (50.0 50.0 64.0)) :`End` (+ (* (`KismetMathLibrary.MakeVector` (`KismetMathLibrary.Conv_IntToDouble` (`self.PX`)) (`KismetMathLibrary.Conv_IntToDouble` (`self.PY`))) 100.0) (50.0 50.0 64.0)) :`TraceChannel` "TraceTypeQuery1" :`DrawDebugType` "ForDuration"))

(fn `UserConstructionScript`)