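; Turn-based battle HUD that draws unit status over the 3D scene on the canvas.
; Units found by a sphere trace around the player pawn get small health, power and movement bars.
; The selected unit instead gets a large material-drawn panel with name, segmented bars and turn-arrow hitboxes that highlight on hover and rotate it on click.
; Dot-product checks against the camera skip units behind it.
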(event `self.ReceiveDrawHUD`
  (params (SizeX :type Integer) (SizeY :type Integer))
  (bind (_x _y) (`self.HealthCounterOffsetReturn`))
  (bind (_x_2 _y_2) (`self.TurnLeftArrowOffsetReturn`))
  (bind (_x_3 _y_3) (`self.TurnRightArrowOffsetReturn`))
  (bind (_x_4 _y_4) (`self.TurnLeftArrowOffsetReturn`))
  (bind (_x_5 _y_5) (`self.TurnRightArrowOffsetReturn`))
  (bind _unittoattachhudelements (`self.UnitToAttachHUDElements`))
  (bind _unittoattachhudelements_2 (`self.UnitToAttachHUDElements`))
  (bind _unittoattachhudelements_3 (`self.UnitToAttachHUDElements`))
  (bind _unittoattachhudelements_4 (`self.UnitToAttachHUDElements`))
  (bind (_x_6 _y_6) (`KismetMathLibrary.BreakVector2D` (`self.MovementBarOffset`)))
  (bind (_x_7 _y_7) (`KismetMathLibrary.BreakVector2D` (`self.MovementBarDimensions`)))
  (bind (_x_8 _y_8) (`KismetMathLibrary.BreakVector2D` (`self.HealthBarOffset`)))
  (bind (_x_9 _y_9) (`KismetMathLibrary.BreakVector2D` (`self.HealthBarDimensions`)))
  (bind (_x_10 _y_10) (`KismetMathLibrary.BreakVector2D` (`self.MovementBarOffset`)))
  (bind (_x_11 _y_11) (`KismetMathLibrary.BreakVector2D` (`self.MovementBarDimensions`)))
  (bind (_x_12 _y_12) (`KismetMathLibrary.BreakVector2D` (`self.MovementBarOffset`)))
  (bind (_x_13 _y_13) (`KismetMathLibrary.BreakVector2D` (`self.MovementBarDimensions`)))
  (bind (_x_14 _y_14) (`KismetMathLibrary.BreakVector2D` (`self.PowerBarOffset`)))
  (bind (_x_15 _y_15) (`KismetMathLibrary.BreakVector2D` (`self.PowerBarDimensions`)))
  (bind _numberofmoves (`/Game/Battle/Core/Units/Unit.NumberOfMoves` (`self.UnitToAttachHUDElements`)))
  (bind _camera1 (`/Game/Battle/Core/Blueprints/Game/TBS_PlayerPawn.Camera1` (`self.StoredPlayer`)))
  (bind _returnvalue (/ (`/Game/Battle/Core/Units/Unit.CurrentHealth` _unittoattachhudelements_3) (`/Game/Battle/Core/Units/Unit.Health` _unittoattachhudelements_3)))
  (bind _returnvalue_2 (/ (`/Game/Battle/Core/Units/Unit.CurrentPower` _unittoattachhudelements_4) (`/Game/Battle/Core/Units/Unit.Power` _unittoattachhudelements_4)))
  (bind _returnvalue_3 (* (`/Game/Battle/Core/Units/Unit.NumberOfMoves` _unittoattachhudelements_2) (`/Game/Battle/Core/Units/Unit.MovementRange` _unittoattachhudelements_2)))
  (bind _returnvalue_4 (/ (`KismetMathLibrary.Conv_IntToDouble` (`/Game/Battle/Core/Units/Unit.CurrentMovementRange` _unittoattachhudelements)) (`KismetMathLibrary.Conv_IntToDouble` (* (`/Game/Battle/Core/Units/Unit.MovementRange` _unittoattachhudelements) (`/Game/Battle/Core/Units/Unit.NumberOfMoves` _unittoattachhudelements)))))
  ;[1 1 1] Only draw the larger HUD element if 1) Unit to Attach HUDElements is not Null, and 2) it is not behind the camera.
  (`self.MinorPanes`) ; Start by drawing all the minor panes
  (if (not (!= (`self.StoredPlayer`) null))
    (bind _astbs_player_pawn (cast `/Game/Battle/Core/Blueprints/Game/TBS_PlayerPawn` (`GameplayStatics.GetPlayerPawn` 0)))
    (set `self.StoredPlayer` _astbs_player_pawn))
  (if (!= (`self.UnitToAttachHUDElements`) null)
    (if (> (`KismetMathLibrary.Dot_VectorVector` (`KismetMathLibrary.Normal` (- (`self.K2_GetActorLocation` (`self.UnitToAttachHUDElements`)) (`SceneComponent.K2_GetComponentLocation` _camera1))) (`KismetMathLibrary.Conv_RotatorToVector` (`SceneComponent.K2_GetComponentRotation` _camera1))) 0.0)
      ;[1 1 1] Setting some reusable values
      (set `self.UnitHUDOrigin_X` (- (.x (`self.Project` (+ (`self.K2_GetActorLocation` (`self.UnitToAttachHUDElements`)) (`self.HUD_Offset`)))) (/ (`self.UnitHUD_Width`) 2.0)))
      (set `self.UnitHUDOrigin_Y` (.y (`self.Project` (+ (`self.K2_GetActorLocation` (`self.UnitToAttachHUDElements`)) (`self.HUD_Offset`)))))
      ;[1 1 1] Background bit
      (`self.DrawMaterial` (`self.HUDMat`) (`self.UnitHUDOrigin_X`) (`self.UnitHUDOrigin_Y`) (`self.UnitHUD_Width`) (`self.UnitHUD_Height`) 0.0 0.25 1.0 0.25)
      ;[1 1 1] Left and Right arrows
      (`self.DrawMaterial` (`self.HUDMat`) _x_4 _y_4 48.0 48.0 0.0 0.0 0.128 0.125)
      (`self.AddHitBox` (`KismetMathLibrary.MakeVector2D` _x_2 _y_2) (48.0 48.0) "Left" true)
      (`self.DrawMaterial` (`self.HUDMat`) _x_5 _y_5 48.0 48.0 0.125 0.0 0.125 0.125)
      (`self.AddHitBox` (`KismetMathLibrary.MakeVector2D` _x_3 _y_3) (48.0 48.0) "Right" true)
      ;[1 1 1] Unit Name
      (`self.DrawText` (`KismetSystemLibrary.GetDisplayName` (`self.UnitToAttachHUDElements`)) (struct :`A` 1.0) _x _y "/Game/Battle/Core/Blueprints/HUD/RobotoDistanceField.RobotoDistanceField")
      ;[1 1 1] Movement Bar
      (`self.DrawMaterial` (`self.HUDMat`) (+ (`self.UnitHUDOrigin_X`) _x_6) (+ (`self.UnitHUDOrigin_Y`) _y_6) (* _returnvalue_4 _x_7) _y_7 0.0 0.9375 _returnvalue_4 0.0625)
      ;[1 1 1] Health Bar
      (`self.DrawMaterial` (`self.HUDMat`) (+ (`self.UnitHUDOrigin_X`) _x_8) (+ (`self.UnitHUDOrigin_Y`) _y_8) (* _returnvalue _x_9) _y_9 0.0 0.875 (* _returnvalue 0.5) 0.0625)
      ;[1 1 1] Power Bar
      (`self.DrawMaterial` (`self.HUDMat`) (+ (`self.UnitHUDOrigin_X`) _x_14) (+ (`self.UnitHUDOrigin_Y`) _y_14) (* _returnvalue_2 _x_15) _y_15 0.5 0.875 (* _returnvalue_2 0.5) 0.0625)
      ;[1 1 1] Movement Bar segements
      (for _index (range 1 _returnvalue_3)
        (`self.DrawRect` (struct :`B` 0.976471 :`A` 1.0) (+ (+ (`self.UnitHUDOrigin_X`) _x_10) (- (* (`KismetMathLibrary.Conv_IntToDouble` _index) (/ _x_11 (`KismetMathLibrary.Conv_IntToDouble` _returnvalue_3))) 1.0)) (+ _y_10 (`self.UnitHUDOrigin_Y`)) 2.0 (* _y_11 0.5)))
      (for _index_2 (range 1 _numberofmoves)
        (`self.DrawRect` (struct :`B` 1.0 :`A` 1.0) (+ (+ (`self.UnitHUDOrigin_X`) _x_12) (- (* (`KismetMathLibrary.Conv_IntToDouble` _index_2) (/ _x_13 (`KismetMathLibrary.Conv_IntToDouble` _numberofmoves))) 2.0)) (+ _y_12 (`self.UnitHUDOrigin_Y`)) 4.0 _y_13)))))

(event `SelectedUnit`
  ;[1 1 1] The unit to attach the bigger HUD element to, called from the TBS player controller.
  (bind _asmain_player_controller (cast `/Game/Battle/Core/Blueprints/Game/MainPlayerController` (`GameplayStatics.GetPlayerController` 0)))
  (set `self.UnitToAttachHUDElements` (`/Game/Battle/Core/Blueprints/Game/MainPlayerController.Selected_toUnit` _asmain_player_controller)))

(event `DeselectUnit`
  ;[1 1 1] Clearing the unit to attach the bigger HUD element to.
  (set `self.UnitToAttachHUDElements` null))

(event `self.ReceiveHitBoxBeginCursorOver`
  (params (BoxName :type Name))
  (bind _hudmat (`self.HUDMat`))
  (bind _hudmat_2 (`self.HUDMat`))
  ;[1 1 1] Highlight the Right Arrow on the big unit HUD element on mouse over.
  (switch `name` BoxName
    (:`Left`
      (`MaterialInstanceDynamic.SetScalarParameterValue` _hudmat "EnableLeft" 1.0)
      (`MaterialInstanceDynamic.SetVectorParameterValue` _hudmat "LeftArrowCollor" (struct :`G` 1.0 :`A` 1.0)))
    (:`Right`
      (`MaterialInstanceDynamic.SetScalarParameterValue` _hudmat_2 "EnableRight" 1.0)
      (`MaterialInstanceDynamic.SetVectorParameterValue` _hudmat_2 "RightArrowCollor" (struct :`G` 1.0 :`A` 1.0)))))

(event `self.ReceiveHitBoxEndCursorOver`
  (params (BoxName :type Name))
  (bind _hudmat (`self.HUDMat`))
  (bind _hudmat_2 (`self.HUDMat`))
  ;[1 1 1] Highlight the Left Arrow on the big unit HUD element on mouse over.
  (switch `name` BoxName
    (:`Left`
      (`MaterialInstanceDynamic.SetScalarParameterValue` _hudmat_2 "EnableLeft" 0.0)
      (`MaterialInstanceDynamic.SetVectorParameterValue` _hudmat_2 "LeftArrowCollor" (struct :`B` 1.0 :`A` 1.0)))
    (:`Right`
      (`MaterialInstanceDynamic.SetScalarParameterValue` _hudmat "EnableRight" 0.0)
      (`MaterialInstanceDynamic.SetVectorParameterValue` _hudmat "RightArrowCollor" (struct :`B` 1.0 :`A` 1.0)))))

(event `self.ReceiveHitBoxClick`
  (params (BoxName :type Name))
  ;[1 1 1] Send turn left/right to the unit from the big unit HUD element
  (switch `name` BoxName
    (:`Left`
      (`/Game/Battle/Core/Units/Unit.TurnUnit` (`self.UnitToAttachHUDElements`) -1))
    (:`Right`
      (`/Game/Battle/Core/Units/Unit.TurnUnit` (`self.UnitToAttachHUDElements`) 1))))

(fn `MinorPanes`
  (returns (Done :type Boolean))
  (bind _returnvalue (`self.K2_GetActorLocation` (`GameplayStatics.GetPlayerPawn` 0)))
  ;[1 1 1] Get the units within 4500 cm/uu of the player pawn by using a multi sphere trace. Set Actors for Minor Panes populates the array "Actors for Panes"
  (bind _outhits (`KismetSystemLibrary.SphereTraceMultiForObjects` _returnvalue (+ _returnvalue (0.0 0.0 50.0)) 4500.0 (`self.FindPawns`)))
  (`self.SetActorsForMinorPanes` _outhits)
  (bind _astbs_player_pawn (cast `/Game/Battle/Core/Blueprints/Game/TBS_PlayerPawn` (`GameplayStatics.GetPlayerPawn` 0)))
  ;[1 1 1] Loop through all the units
  (for _array_element (`self.ActorsForPanes`)
    ;[1 1 1] If the unit is hidded, don't draw the element
    (if (not (`Actor.bHidden` _array_element))
      (bind _camera1 (`/Game/Battle/Core/Blueprints/Game/TBS_PlayerPawn.Camera1` _astbs_player_pawn))
      ;[1 1 1] Get's the dot product of the unit (location - camera location) and the camera's rotation. Prevents the little HUD elements from rendering when the unit is behind the camera
      (if (> (`KismetMathLibrary.Dot_VectorVector` (`KismetMathLibrary.Normal` (- (`self.K2_GetActorLocation` _array_element) (`SceneComponent.K2_GetComponentLocation` _camera1))) (`KismetMathLibrary.Conv_RotatorToVector` (`SceneComponent.K2_GetComponentRotation` _camera1))) 0.0)
        ;[1 1 1] Prevents the smaller HUD element from rendering on the selected unit as it has the large element
        (bind _asunit (cast `/Game/Battle/Core/Units/Unit` _array_element))
        (if (!= (`self.UnitToAttachHUDElements`) _asunit)
          (bind _y (.y (`self.Project` (+ (`self.K2_GetActorLocation` _array_element) (0.0 0.0 100.0)))))
          (bind _returnvalue_2 (- (.x (`self.Project` (+ (`self.K2_GetActorLocation` _array_element) (0.0 0.0 100.0)))) 32.0))
          ;[1 1 1] Rendering the Health, Power, and Movement bars for the unit
          (`self.DrawRect` (struct :`R` 1.0 :`A` 1.0) _returnvalue_2 _y (* (/ (`/Game/Battle/Core/Units/Unit.CurrentHealth` _asunit) (`/Game/Battle/Core/Units/Unit.Health` _asunit)) 64.0) 4.0)
          (`self.DrawRect` (struct :`B` 1.0 :`A` 1.0) _returnvalue_2 (+ _y 4.0) (* (/ (`/Game/Battle/Core/Units/Unit.CurrentPower` _asunit) (`/Game/Battle/Core/Units/Unit.Power` _asunit)) 64.0) 4.0)
          (`self.DrawRect` (struct :`R` 1.0 :`G` 1.0 :`A` 1.0) _returnvalue_2 (+ _y 8.0) (* (/ (`KismetMathLibrary.Conv_IntToDouble` (`/Game/Battle/Core/Units/Unit.CurrentMovementRange` _asunit)) (`KismetMathLibrary.Conv_IntToDouble` (* (`/Game/Battle/Core/Units/Unit.MovementRange` _asunit) (`/Game/Battle/Core/Units/Unit.NumberOfMoves` _asunit)))) 64.0) 4.0)))))
  (return true))

(fn `SetActorsForMinorPanes`
  (params (HitsIn :type "Array of HitResult Structure"))
  (returns (Out :type Boolean))
  (locals (TempString :type String))
  (`KismetArrayLibrary.Array_Clear` (`self.ActorsForPanes`))
  (for (_array_element _array_index) HitsIn
    (`KismetArrayLibrary.Array_Set` (`self.ActorsForPanes`) _array_index (`.HitActor` (`GameplayStatics.BreakHitResult` _array_element)) true))
  (return true))

(fn `UserConstructionScript`
  ;[1 1 1] Create the DMI for the HUD and then set the max # of units for the small HUD elements
  (bind _returnvalue (`KismetMaterialLibrary.CreateDynamicMaterialInstance` "/Game/Battle/Core/Blueprints/HUD/UnitHUDMaterial.UnitHUDMaterial"))
  (set `self.HUDMat` _returnvalue)
  (`KismetArrayLibrary.Array_Resize` (`self.ActorsForPanes`) 50))