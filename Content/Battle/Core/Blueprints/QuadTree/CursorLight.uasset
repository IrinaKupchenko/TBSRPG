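; Cursor-following light actor that the Player Controller moves toward the mouse's world position via MoveMe, using interpolated movement.
; It crossfades two point lights, intended as shadow-casting and non-shadow, with a timeline that plays when the player's Unit pawn begins overlapping and reverses when it leaves.
; BeginPlay sets the starting light from the sphere overlap, overlap events also toggle shadow casting, and the construction script matches the second light's color to the first.
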(event `self.ReceiveBeginPlay`
  (bind _pointlight1 (`self.PointLight1`))
  ;[1 1 1] Is the player pawn overlapping me at the start of play? If yes, shadow light on/non-shadow light off; if false, shadow light off/non-shadow light on.
  (bind _asunit (cast `/Game/Battle/Core/Units/Unit` (`GameplayStatics.GetPlayerPawn` 0)))
  (set `self.UnitReference` _asunit)
  (if (!= (`PrimitiveComponent.IsOverlappingActor` (`self.Sphere1`) (`GameplayStatics.GetPlayerPawn` 0)) false)
    (`LightComponent.SetCastShadows` _pointlight1 true)
    (`LightComponent.SetIntensity` _pointlight1 (`self.DefaultBrightness`))
    (`LightComponent.SetIntensity` (`self.PointLight2`) 0.0)
    (else
      (`LightComponent.SetIntensity` (`self.PointLight2`) (`self.DefaultBrightness`))
      (`LightComponent.SetIntensity` (`self.PointLight1`) 0.0))))

(event `self.ReceiveActorBeginOverlap`
  (params (OtherActor :type "Actor Object Reference"))
  ;[1 1 1] If the player pawn overlaps me then fade in the shadow casting light and fade out the non-shadow casting light. When the player pawn stops overlapping me, reverse this process
  (if (== OtherActor (`self.UnitReference`))
    (`LightComponent.SetCastShadows` (`self.PointLight1`) false)
    (bind (_direction _alpha) (`Timeline|FadeTimeline` :!label _label)
      (:`Update`
        (bind _returnvalue (`KismetMathLibrary.Lerp` 0.0 (`self.DefaultBrightness`) _alpha))
        (`LightComponent.SetIntensity` (`self.PointLight1`) _returnvalue)
        (`LightComponent.SetIntensity` (`self.PointLight2`) (- (`self.DefaultBrightness`) _returnvalue)))
      (:`Finished`
        (if (`|EnumEquality` _direction "Backward")
          (`LightComponent.SetCastShadows` (`self.PointLight1`) false))))))

(event `self.ReceiveActorEndOverlap`
  (params (OtherActor :type "Actor Object Reference"))
  ;[1 1 1] If the player pawn overlaps me then fade in the shadow casting light and fade out the non-shadow casting light. When the player pawn stops overlapping me, reverse this process
  (if (== (stale `self.ReceiveActorBeginOverlap` OtherActor) (`self.UnitReference`))
    (`LightComponent.SetCastShadows` (`self.PointLight1`) true)
    (goto _label :!via `Reverse`)))

(event `MoveMe`
  (params (Target :type "Vector Structure"))
  ;[1 1 1] Called from the Player Controller to move the light to what the mouse is overlapping in the world.
  (`self.K2_SetActorLocation` (`KismetMathLibrary.VInterpTo` (`self.K2_GetActorLocation`) Target (`GameplayStatics.GetWorldDeltaSeconds`) 2.0)))

(fn `UserConstructionScript`
  ;[1 1 1] Set light 2's color to that of light 1
  (`LightComponent.SetLightColor` (`self.PointLight2`) (`KismetMathLibrary.Conv_ColorToLinearColor` (`LightComponentBase.LightColor` (`self.PointLight1`))) true))