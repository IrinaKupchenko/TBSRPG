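; TriggeredLight is a light actor that casts shadows only while the player pawn (TBS_PlayerPawn) is nearby, likely to save shadow cost.
; Two point lights share a random yellowish colour drawn from the TBS_Game MainStream at construction.
; BeginPlay picks the active light from sphere overlaps.
; Begin and end overlap play or reverse a timeline crossfading between shadowed and unshadowed lights, disabling shadows once faded back.
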(event `self.ReceiveBeginPlay`
  (bind _pointlight1 (`self.PointLight1`))
  ;[1 1 1] Is the player pawn overlapping me at the start of play? If yes, shadow light on/non-shadow light off; if false, shadow light off/non-shadow light on.
  (if (> (`KismetArrayLibrary.Array_Length` (`PrimitiveComponent.GetOverlappingActors` (`self.Sphere1`) "/Game/Battle/Core/Blueprints/Game/TBS_PlayerPawn.TBS_PlayerPawn_C")) 0)
    (`LightComponent.SetCastShadows` _pointlight1 true)
    (`LightComponent.SetIntensity` _pointlight1 (`self.DefaultBrightness`))
    (`LightComponent.SetIntensity` (`self.PointLight2`) 0.0)
    (else
      (`LightComponent.SetIntensity` (`self.PointLight2`) (`self.DefaultBrightness`))
      (`LightComponent.SetIntensity` (`self.PointLight1`) 0.0))))

(event `self.ReceiveActorBeginOverlap`
  (params (OtherActor :type "Actor Object Reference"))
  ;[1 1 1] If the player pawn overlaps me then fade in the shadow casting light and fade out the non-shadow casting light. When the player pawn stops overlapping me, reverse this process
  (cast `/Game/Battle/Core/Blueprints/Game/TBS_PlayerPawn` OtherActor)
  (`LightComponent.SetCastShadows` (`self.PointLight1`) true)
  (bind (_direction _alpha) (`Timeline|FadeTimeline` :!label _label)
    (:`Update`
      (bind _returnvalue (`KismetMathLibrary.Lerp` 0.0 (`self.DefaultBrightness`) _alpha))
      (`LightComponent.SetIntensity` (`self.PointLight1`) _returnvalue)
      (`LightComponent.SetIntensity` (`self.PointLight2`) (- (`self.DefaultBrightness`) _returnvalue)))
    (:`Finished`
      (if (`|EnumEquality` _direction "Backward")
        (`LightComponent.SetCastShadows` (`self.PointLight1`) false)))))

(event `self.ReceiveActorEndOverlap`
  (params (OtherActor :type "Actor Object Reference"))
  ;[1 1 1] If the player pawn overlaps me then fade in the shadow casting light and fade out the non-shadow casting light. When the player pawn stops overlapping me, reverse this process
  (cast `/Game/Battle/Core/Blueprints/Game/TBS_PlayerPawn` OtherActor)
  (goto _label :!via `Reverse`))

(fn `UserConstructionScript`
  (bind _pointlight1 (`self.PointLight1`))
  (bind _mainstream (`/Game/Battle/Core/Blueprints/Game/TBS_Game.MainStream` (`self.GameMode`)))
  ;[1 1 1] Get the game mode to use the Random Stream from it
  (bind _astbs_game (cast `/Game/Battle/Core/Blueprints/Game/TBS_Game` (`GameplayStatics.GetGameMode`)))
  (set `self.GameMode` _astbs_game)
  ;[1 1 1] Set the lights' colors to a random yellowish hue using the random stream from the game mode.
  (`LightComponent.SetLightColor` _pointlight1 (`KismetMathLibrary.MakeColor` (`KismetMathLibrary.RandomFloatInRangeFromStream` 0.7 0.9 _mainstream) (`KismetMathLibrary.RandomFloatInRangeFromStream` 0.5 0.6 _mainstream) (`KismetMathLibrary.RandomFloatInRangeFromStream` 0.0 0.2 _mainstream)) true)
  (`LightComponent.SetLightColor` (`self.PointLight2`) (`KismetMathLibrary.Conv_ColorToLinearColor` (`LightComponentBase.LightColor` _pointlight1)) true))