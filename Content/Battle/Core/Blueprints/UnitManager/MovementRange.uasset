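; Turn-based battle actor that displays a movement range as instanced grid tiles, with show and hide toggles.
; SimplePopulate sphere-traces nearby grid objects, keeps cells the pathfinder accepts, then flood-fills outward by neighbor offsets, capping step count at the range.
; PopulateGrid instead places tiles from a supplied location list.
; A dynamic MoveArea material, created at construction, receives the range as MaxDistance.
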(event `ShowRange`
  (`SceneComponent.SetVisibility` true))

(event `HideRange`
  (`SceneComponent.SetVisibility` false))

(fn `PopulateGrid`
  (params (Locations :type "Array of Vector Structure"))
  (for _array_element Locations
    (`InstancedStaticMeshComponent.AddInstance` (`KismetMathLibrary.Conv_VectorToTransform` _array_element)))
  (`self.ShowRange`))

(fn `SetRange`
  (params (Range :type "Float (double-precision)"))
  (`MaterialInstanceDynamic.SetScalarParameterValue` (`self.MaterialRef`) "MaxDistance" Range))

(fn `SimplePopulate`
  (params (Location :type "Vector Structure") (Range :type "Float (double-precision)"))
  (bind _moveindex (`self.MoveIndex`))
  (`InstancedStaticMeshComponent.ClearInstances`)
  (`KismetArrayLibrary.Array_Clear` (`self.MoveIndex`))
  (`KismetArrayLibrary.Array_Clear` (`self.FinalLocations`))
  (`KismetArrayLibrary.Array_Clear` (`self.NavTestedLocations`))
  (`self.SetRange` Range)
  (bind _outhits (`KismetSystemLibrary.SphereTraceMultiForObjects` Location (+ Location (0.0 0.0 2.0)) (* Range 100.0) (`|MakeArray` "ObjectTypeQuery7" :!type "EObjectTypeQuery Enum")))
  (for _array_element _outhits
    (bind _returnvalue (`self.K2_GetActorLocation` (`.HitActor` (`GameplayStatics.BreakHitResult` _array_element))))
    (bind _returm (`/Game/Battle/Core/Blueprints/A-Star/PathFinder.ReturnGridStatus` (`self.PathFinderRef`) _returnvalue))
    (if (>= _returm 0)
      (`KismetArrayLibrary.Array_Add` (`self.NavTestedLocations`) _returnvalue)))
  (`KismetArrayLibrary.Array_Add` (`self.MoveIndex`))
  (`KismetArrayLibrary.Array_Add` (`self.FinalLocations`) Location)
  (for (_ _array_index) (`self.NavTestedLocations`)
    (if (>= (- (`KismetArrayLibrary.Array_Length` (`self.MoveIndex`)) 1) _array_index)
      (for _array_element_2 (`self.TestLocations`)
        (bind _returnvalue_2 (+ _array_element_2 (`|GetArrayItem` (`self.FinalLocations`) _array_index)))
        (if (and (not (`KismetArrayLibrary.Array_Contains` (`self.FinalLocations`) _returnvalue_2)) (`KismetArrayLibrary.Array_Contains` (`self.NavTestedLocations`) _returnvalue_2) (< (`|GetArrayItem` (`self.MoveIndex`) _array_index) (`KismetMathLibrary.FFloor` Range)))
          (`KismetArrayLibrary.Array_Add` (`self.FinalLocations`) _returnvalue_2)
          (`KismetArrayLibrary.Array_Add` _moveindex (+ (`|GetArrayItem` _moveindex _array_index) 1))
          (`InstancedStaticMeshComponent.AddInstance` (`KismetMathLibrary.Conv_VectorToTransform` (+ (- _returnvalue_2 (`self.K2_GetActorLocation`)) (0.0 0.0 5.0))))))))
  (`self.ShowRange`))

(fn `UserConstructionScript`
  (bind _astbs_game (cast `/Game/Battle/Core/Blueprints/Game/TBS_Game` (`GameplayStatics.GetGameMode`)))
  (set `self.PathFinderRef` (`/Game/Battle/Core/Blueprints/Game/TBS_Game.PathFinderActorReference` _astbs_game))
  (bind _returnvalue (`PrimitiveComponent.CreateDynamicMaterialInstance` 0 "/Game/Battle/Core/Materials/Interface/MoveArea.MoveArea"))
  (set `self.MaterialRef` _returnvalue)
  (`PrimitiveComponent.SetMaterial` (`self.Range`) 0 _returnvalue))