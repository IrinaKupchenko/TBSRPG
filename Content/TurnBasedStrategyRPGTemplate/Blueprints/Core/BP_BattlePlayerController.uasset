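; BP_BattlePlayerController is the battle player controller that replaces the default mouse cursor with a dynamic UMG cursor.
; On BeginPlay it creates the cursor widget at high Z-order and hides the default cursor behind an empty cursor widget.
; BP_Grid events set the widget's type and angle, passing along ability, spell and character context.
; Tick moves the widget to the DPI-scaled mouse position.
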(event `self.ReceiveBeginPlay`
  ;[1 1 1] Set cursor events
  (bind _returnvalue (`GameplayStatics.GetActorOfClass` "/Game/TurnBasedStrategyRPGTemplate/Blueprints/Grid/BP_Grid.BP_Grid_C"))
  (bind _output_get (set `self.grid` _returnvalue))
  (add `/Game/TurnBasedStrategyRPGTemplate/Blueprints/Grid/BP_Grid.OnCursorChanged` _output_get (delegate `OnCursorChangedHandler`))
  (add `/Game/TurnBasedStrategyRPGTemplate/Blueprints/Grid/BP_Grid.OnCursorAngleChanged` (`self.grid`) (delegate `OnCursorAngleChangedHandler`))
  (bind _returnvalue_2 (`|CreateWidget` "/Game/TurnBasedStrategyRPGTemplate/Blueprints/Widgets/WBP_BattleCursor.WBP_BattleCursor_C"))
  (bind _output_get_2 (set `self.cursorWidget` _returnvalue_2))
  (`UserWidget.AddToViewport` _output_get_2 999)
  (bind _returnvalue_3 (`|CreateWidget` "/Game/TurnBasedStrategyRPGTemplate/Blueprints/Widgets/WBP_EmptyMouseCursor.WBP_EmptyMouseCursor_C"))
  (`self.SetMouseCursorWidget` "Default" _returnvalue_3))

(event `OnCursorAngleChangedHandler`
  (params (angle :type "Float (double-precision)"))
  ;[1 1 1] Set cursor events
  (`/Game/TurnBasedStrategyRPGTemplate/Blueprints/Widgets/WBP_BattleCursor.SetCursorAngle` (`self.cursorWidget`) angle))

(event `OnCursorChangedHandler`
  (params (cursorType :type "/Game/TurnBasedStrategyRPGTemplate/Blueprints/Enums/E_BattleCursorType Enum" :default "NewEnumerator0") (activeAbility :type "/Game/TurnBasedStrategyRPGTemplate/Blueprints/Abilities/ActiveAbilities/BP_ActiveAbilityBase Object Reference") (spell :type "/Game/TurnBasedStrategyRPGTemplate/Blueprints/Spells/BP_SpellBase Object Reference") (character :type "/Game/TurnBasedStrategyRPGTemplate/Blueprints/Units/Characters/BP_CharacterBase Class Reference"))
  (bind _cursorwidget (`self.cursorWidget`))
  ;[1 1 1] Set cursor events
  (`/Engine/EditorBlueprintResources/StandardMacros.IsValid` _cursorwidget
    (:`Is Valid`
      (`/Game/TurnBasedStrategyRPGTemplate/Blueprints/Widgets/WBP_BattleCursor.ChangeCursor` _cursorwidget cursorType activeAbility spell character))))

(event `self.ReceiveTick`
  (params (DeltaSeconds :type "Float (single-precision)"))
  (bind _cursorwidget (`self.cursorWidget`))
  (bind (_locationx _locationy) (`WidgetLayoutLibrary.GetMousePositionScaledByDPI` self))
  ;[1 1 1] Keep the cursor widget on mouse location
  (`/Engine/EditorBlueprintResources/StandardMacros.IsValid` _cursorwidget
    (:`Is Valid`
      (`UserWidget.SetPositionInViewport` _cursorwidget (`KismetMathLibrary.MakeVector2D` _locationx _locationy) false))))

(fn `UserConstructionScript`)